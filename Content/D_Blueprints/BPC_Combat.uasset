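; Player combat component that implements a toggleable target lock for BP_ThirdPersonCharacter.
; IA_Lock runs a debug-drawn sphere trace for pawns toward a point ahead of the camera, storing any hit and attaching a BP_TargetLockWidget actor to it.
; While locked, movement follows controller rotation and Tick aims control rotation at the target with a downward pitch offset.
; Pressing again clears the target, destroys the marker and restores orient-to-movement.
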(event Input|EnhancedActionEvents|EnhancedInputActionIA_Lock
  (params (ActionValue :type Boolean) (ElapsedSeconds :type Float%20%28double-precision%29) (TriggeredSeconds :type Float%20%28double-precision%29) (InputAction :type Input%20Action%20Object%20Reference :default "/Game/ThirdPerson/Input/Actions/IA_Lock.IA_Lock"))
  (bind _returnvalue (Game|GetPlayerCameraManager 0))
  (bind _player_bp (Variables|Default|GetPlayer-BP))
  (bind _player_bp_2 (Variables|Default|GetPlayer-BP))
  (bind _transformcomponent (Variables|/Script/Engine.PlayerCameraManager|GetTransformComponent _returnvalue))
  (bind _charactermovement (Variables|/Script/Engine.Character|GetCharacterMovement _player_bp))
  (bind _charactermovement_2 (Variables|/Script/Engine.Character|GetCharacterMovement _player_bp_2))
  (bind _returnvalue_2 (Transformation|GetWorldLocation _transformcomponent))
  ;[0.15 0.15 0.15 0.5] Target Lock
  (:Started
    (Variables|Default|GetTargetLock-Actor
      (:then
        (Variables|Default|SetTargetLock-Actor 0)
        (Variables|/Script/Engine.CharacterMovementComponent|SetbOrientRotationToMovement _charactermovement true)
        (Variables|/Script/Engine.CharacterMovementComponent|SetbUseControllerDesiredRotation _charactermovement false)
        (Actor|DestroyActor (Variables|Default|GetTargetLock-Widget)))
      (:else
        (bind (_outhit _returnvalue_3) (Collision|SphereTraceForObjects "0, 0, 0" (+ (Math|Vector|MakeVector (.x _returnvalue_2) (.y _returnvalue_2) (+ (.z _returnvalue_2) 2e+01)) (* (Math|Vector|GetForwardVector (Transformation|GetWorldRotation _transformcomponent)) 1e+03)) 1.5e+02 (Utilities|Array|MakeArray "ObjectTypeQuery3") false 0 "ForDuration" true "(R=1.000000,G=0.000000,B=0.000000,A=1.000000)" "(R=0.000000,G=1.000000,B=0.000000,A=1.000000)" 2.0))
        (if _returnvalue_3
          (Variables|Default|SetTargetLock-Actor (.HitActor (Collision|BreakHitResult _outhit)))
          (Variables|/Script/Engine.CharacterMovementComponent|SetbOrientRotationToMovement _charactermovement_2 false)
          (Variables|/Script/Engine.CharacterMovementComponent|SetbUseControllerDesiredRotation _charactermovement_2 true)
          (bind _returnvalue_4 (Game|SpawnActorfromClass "/Game/D_Blueprints/BP_TargetLockWidget.BP_TargetLockWidget_C" (Math|Transform|MakeTransform (Math|Vector|MakeVector (.x (.location (Transformation|GetActorTransform (Variables|Default|GetTargetLock-Actor)))) (.y (.location (Transformation|GetActorTransform (Variables|Default|GetTargetLock-Actor)))) (+ (.z (.location (Transformation|GetActorTransform (Variables|Default|GetTargetLock-Actor)))) 2e+01)) (.rotation (Transformation|GetActorTransform (Variables|Default|GetTargetLock-Actor))) "1.000000,1.000000,1.000000") "AlwaysSpawn" "MultiplyWithRoot" 0 0))
          (bind _output_get (Variables|Default|SetTargetLock-Widget _returnvalue_4))
          (Transformation|AttachActorToActor _output_get (Variables|Default|GetTargetLock-Actor) "None" "SnapToTarget" "SnapToTarget" "SnapToTarget" true))))))

(event EventTick
  (params (DeltaSeconds :type Float%20%28single-precision%29))
  (bind _player_bp (Variables|Default|GetPlayer-BP))
  (bind _targetlock_actor (Variables|Default|GetTargetLock-Actor))
  (bind _returnvalue (Transformation|GetActorLocation _targetlock_actor))
  (bind _returnvalue_2 (Transformation|GetActorLocation _player_bp))
  (bind _returnvalue_3 (Math|Rotator|FindLookatRotation _returnvalue_2 _returnvalue))
  ;[0.15 0.15 0.15 0.5] Target Lock
  ;;[0.15 0.15 0.15 0.5] Target Lock Update
  (Variables|Default|GetTargetLock-Actor
    (:then
      (Pawn|SetControlRotation (Pawn|GetController _player_bp) (Math|Rotator|MakeRotator (.roll _returnvalue_3) (+ (.pitch _returnvalue_3) -2e+01) (.yaw _returnvalue_3))))
    (:else)))

(event EventBeginPlay
  ;[0.15 0.15 0.15 0.5] Get Player CLass
  (bind _asbp_third_person_character (Utilities|Casting|CastToBP_ThirdPersonCharacter (Components|GetOwner)))
  (Variables|Default|SetPlayer-BP _asbp_third_person_character))